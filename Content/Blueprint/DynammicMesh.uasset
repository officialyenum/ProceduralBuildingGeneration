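; Actor that procedurally builds a simple mesh at BeginPlay with Geometry Script: a thin upright slab with a cut-out, plus a flat slab.
; A box in the main DynamicMeshComponent has a smaller, raised cube from a second component boolean-subtracted from it, then the flat box is appended.
; It then passes the result to ReleaseComputeMesh and destroys the second component, which only supplies the cutting tool.
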(event `self.ReceiveBeginPlay`
  (bind _returnvalue (`BaseDynamicMeshComponent.GetDynamicMesh` (`self.DynamicMeshComponent`)))
  (bind _output_get (set `self.Mesh` _returnvalue))
  (bind _returnvalue_2 (`BaseDynamicMeshComponent.GetDynamicMesh` (`self.DynamicMeshComponent1`)))
  (set `self.Mesh_0` _returnvalue_2)
  (bind _returnvalue_3 (`GeometryScriptLibrary_MeshPrimitiveFunctions.AppendBox` _output_get (make `GeometryScriptPrimitiveOptions` "PerFace") (struct) 5.0 100.0 100.0 0 0 0 "Base" null))
  (bind _returnvalue_4 (`GeometryScriptLibrary_MeshPrimitiveFunctions.AppendBox` (`self.Mesh_0`) (struct) (struct) 30.0 30.0 30.0 0 0 0 "Base" null))
  (bind _returnvalue_5 (`GeometryScriptLibrary_MeshBooleanFunctions.ApplyMeshBoolean` _returnvalue_3 (struct) _returnvalue_4 (`KismetMathLibrary.MakeTransform` (0.0 0.0 50.0)) "Subtract" (struct) null))
  (bind _returnvalue_6 (`GeometryScriptLibrary_MeshPrimitiveFunctions.AppendBox` _returnvalue_5 (struct) (struct) 100.0 100.0 5.0 0 0 0 "Base" null))
  (`self.ReleaseComputeMesh` _returnvalue_6)
  (`ActorComponent.K2_DestroyComponent` (`self.DynamicMeshComponent1`)))

(fn `UserConstructionScript`)