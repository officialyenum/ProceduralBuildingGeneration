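; Procedural wall generator actor that builds a box wall with one window or door cutout using Geometry Script.
; On mesh rebuild, it extrudes a square or rounded rectangle and boolean-subtracts it from the box, giving cut faces their own material slot.
; It then optionally bevels polygroup edges with split normals, assigns materials and recomputes scaled UVs.
; The GenerateRoom and SpawnWall functions are empty stubs.
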(event `self.OnRebuildGeneratedMesh`
  (params (TargetMesh :type "DynamicMesh Object Reference"))
  (bind (_wallsize_x _wallsize_y _wallsize_z) (`KismetMathLibrary.BreakVector` (`self.WallSize`)))
  (bind (_cutoutsize_x _cutoutsize_y _cutoutsize_z) (`KismetMathLibrary.BreakVector` (`self.CutOutSize`)))
  (bind (_cutoutsize_x_2 _cutoutsize_y_2) (`KismetMathLibrary.BreakVector` (`self.CutOutSize`)))
  (bind (_cutoutsize_x_3 _cutoutsize_y_3 _cutoutsize_z_2) (`KismetMathLibrary.BreakVector` (`self.CutOutSize`)))
  (set `self.Dynamic Mesh` TargetMesh)
  (`|ExecutionSequence`
    (:`then_0`
      ;[1 1 1] Create Wall
      (`GeometryScriptLibrary_MeshPrimitiveFunctions.AppendBox` (`self.Dynamic Mesh`) (struct) (struct) (* _wallsize_x 2.0) (* _wallsize_y 2.0) _wallsize_z 0 0 0 "Base" null))
    (:`then_1`
      (if (`self.IsCutOutRounded`)
        ;[1 1 1] Create Rounded Cutout For Windows Or Doors
        (bind _returnvalue (`self.AllocateComputeMesh`))
        (bind _returnvalue_2 (`GeometryScriptLibrary_MeshPrimitiveFunctions.AppendRoundRectangleXY` _returnvalue (struct) (`KismetMathLibrary.MakeTransform` (0.0 0.0 0.0) (struct :`Roll` 90.0)) _cutoutsize_x _cutoutsize_z (`self.Corner Radius`) 0 0 (`self.Steps Round`) null))
        (set `self.CutOutMesh` _returnvalue_2)
        (else
          ;[1 1 1] Create Cutout For Windows Or Doors
          (bind _returnvalue_3 (`self.AllocateComputeMesh`))
          (bind _returnvalue_4 (`GeometryScriptLibrary_MeshPrimitiveFunctions.AppendRectangleXY` _returnvalue_3 (struct) (`KismetMathLibrary.MakeTransform` (0.0 0.0 0.0) (struct :`Roll` 90.0)) _cutoutsize_x_3 _cutoutsize_z_2 0 0 null))
          (set `self.CutOutMesh` _returnvalue_4))))
    (:`then_2`
      ;[1 1 1] Extrude Cutout
      (bind _returnvalue_5 (`GeometryScriptLibrary_MeshModelingFunctions.ApplyMeshExtrude_Compatibility_5p0` (`self.CutOutMesh`) (make `GeometryScriptMeshExtrudeOptions` _cutoutsize_y_2 (0.0 1.0 0.0)) null))
      (`GeometryScriptLibrary_MeshMaterialFunctions.RemapMaterialIDs` _returnvalue_5 0 1 null)
      (set `self.CutOutMesh` _returnvalue_5))
    (:`then_3`
      ;[1 1 1] Apply Cut Out Boolean
      (bind _returnvalue_6 (`GeometryScriptLibrary_MeshBooleanFunctions.ApplyMeshBoolean` (`self.Dynamic Mesh`) (struct) (`self.CutOutMesh`) (`KismetMathLibrary.MakeTransform` (`self.CutOutLocation`)) "Subtract" (struct) null))
      (set `self.Dynamic Mesh` _returnvalue_6))
    (:`then_4`
      ;[1 1 1] Do Bevels
      (if (`self.IsBeveled`)
        (bind _returnvalue_7 (`GeometryScriptLibrary_MeshPolygroupFunctions.ComputePolygroupsFromAngleThreshold` (`self.Dynamic Mesh`) (struct) 25.0 2 null))
        (bind _returnvalue_8 (`GeometryScriptLibrary_MeshModelingFunctions.ApplyMeshPolygroupBevel` _returnvalue_7 (make `GeometryScriptMeshBevelOptions` (`self.BevelAmount`)) null))
        (bind _returnvalue_9 (`GeometryScriptLibrary_MeshNormalsFunctions.ComputeSplitNormals` _returnvalue_8 (make `GeometryScriptSplitNormalsOptions` true 25.0) (struct) null))
        (set `self.Dynamic Mesh` _returnvalue_9)))
    (:`then_5`
      ;[1 1 1] Setup Materials
      (`DynamicMeshComponent.ConfigureMaterialSet` (`self.DynamicMeshComponent`) (`|MakeArray` (`self.Wall Material`) (`self.Cutout Material`))))
    (:`then_6`
      ;[1 1 1] RECOMPUTE SCALE AND UVS
      (bind _returnvalue_10 (`GeometryScriptLibrary_MeshUVFunctions.RecomputeMeshUVs` (`self.Dynamic Mesh`) 0 (struct) (struct) null))
      (`GeometryScriptLibrary_MeshUVFunctions.ScaleMeshUVs` _returnvalue_10 0 (`KismetMathLibrary.MakeVector2D` (`self.UV Scale X`) (`self.UV Scale Y`)) (0.0 0.0) (struct) null))))

(fn `GenerateRoom`
  (params (Points :type "Array of IntPoint Structure")))

(fn `SpawnWall`
  (params (`Wall Points` :type "/Game/Blueprint/Data/S_WallPoints Structure")))

(fn `UserConstructionScript`
  (`parent.UserConstructionScript`))