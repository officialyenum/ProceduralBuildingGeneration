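; BP_ROOM is a procedural room actor that lays out four walls in its construction script from Width and Length.
; It adds one wall mesh instance per unit on each side, rotated and spaced by mesh bounds.
; Spacing mostly uses bounds Max.X, but back-wall depth and right-wall steps use Max.Z.
; Selected door and window meshes are assigned but never instanced, and Height is only printed for debugging.
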(fn `UserConstructionScript`
  (bind _length (`self.Length`))
  (bind (_min _max) (`StaticMeshComponent.GetLocalBounds` (`self.WallMesh`)))
  (bind (_min_2 _max_2) (`StaticMeshComponent.GetLocalBounds` (`self.WallMesh`)))
  (set `self.Width` (`self.Width`))
  (set `self.Length` (`self.Length`))
  (set `self.Area` (`self.Area`))
  (`KismetSystemLibrary.PrintString` "Hello" true true (struct :`G` 0.66 :`B` 1.0 :`A` 1.0) 5.0)
  (`StaticMeshComponent.SetStaticMesh` (`self.DoorMesh`) (`self.Select Door Mesh`))
  (`StaticMeshComponent.SetStaticMesh` (`self.WindowMesh`) (`self.Select Window Mesh`))
  (`StaticMeshComponent.SetStaticMesh` (`self.WallMesh`) (`self.Select Wall Mesh`))
  (bind _output_get (set `self.Height` (`self.Height`)))
  (`KismetSystemLibrary.PrintString` (`KismetStringLibrary.Conv_DoubleToString` _output_get))
  (`KismetSystemLibrary.PrintString` (`KismetStringLibrary.Conv_DoubleToString` (`self.Width`)))
  (`KismetSystemLibrary.PrintString` (`KismetStringLibrary.Conv_DoubleToString` (`self.Length`)))
  (`|ExecutionSequence`
    (:`then_0`
      ;[1 1 1] FRONT WALL
      (for _index (range (`KismetMathLibrary.FTrunc` (`self.Width`)))
        (`InstancedStaticMeshComponent.AddInstance` (`self.WallMesh`) (`KismetMathLibrary.MakeTransform` (`KismetMathLibrary.MakeVector` (* _index (.x (`.Max` (`StaticMeshComponent.GetLocalBounds` (`self.WallMesh`))))))) false)))
    (:`then_1`
      ;[1 1 1] BACK WALL
      (for _index_2 (range (`KismetMathLibrary.FTrunc` (`self.Width`)))
        (`InstancedStaticMeshComponent.AddInstance` (`self.WallMesh`) (`KismetMathLibrary.MakeTransform` (`KismetMathLibrary.MakeVector` (+ (* _index_2 (.x _max)) (.x _max)) (- (* (.z _max) _length -1.0) _length)) (struct :`Yaw` 180.0)) false)))
    (:`then_2`
      ;[1 1 1] LEFT WALL
      (for _index_3 (range (`KismetMathLibrary.FTrunc` (`self.Length`)))
        (`InstancedStaticMeshComponent.AddInstance` (`self.WallMesh`) (`KismetMathLibrary.MakeTransform` (`KismetMathLibrary.MakeVector` 0.0 (* (* _index_3 (.x (`.Max` (`StaticMeshComponent.GetLocalBounds` (`self.WallMesh`))))) -1.0)) (struct :`Yaw` -90.0)) false)))
    (:`then_3`
      ;[1 1 1] RIGHT WALL
      (for _index_4 (range (`KismetMathLibrary.FTrunc` (`self.Length`)))
        (`InstancedStaticMeshComponent.AddInstance` (`self.WallMesh`) (`KismetMathLibrary.MakeTransform` (`KismetMathLibrary.MakeVector` (* (.x _max_2) (`self.Width`)) (* (* _index_4 (.z _max_2)) -1.0)) (struct :`Yaw` -90.0)) false)))))